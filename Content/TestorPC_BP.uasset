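; Test Blueprint, apparently a player controller, that compares looping over a native function's int array directly against looping over a cached copy.
; R feeds SpitIntArrayNative straight into a for-each loop, while T stores its result in Caching first.
; Both print every element and call ObserveCurrentTime before and after, bracketing each approach for timing.
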(event `Key|R`
  (params (Key :type "Key Structure"))
  (:`Pressed`
    (`self.ObserveCurrentTime`)
    (for _array_element (`self.SpitIntArray_Native` (`self.ArrayLength`))
      (`KismetSystemLibrary.PrintString` (`KismetStringLibrary.Conv_IntToString` _array_element) true false))
    (`self.ObserveCurrentTime`)))

(event `Key|T`
  (params (Key :type "Key Structure"))
  (:`Pressed`
    (`self.ObserveCurrentTime`)
    (bind _output_get (set `self.Caching` (`self.SpitIntArray_Native` (`self.ArrayLength`))))
    (for _array_element _output_get
      (`KismetSystemLibrary.PrintString` (`KismetStringLibrary.Conv_IntToString` _array_element) true false))
    (`self.ObserveCurrentTime`)))

(fn `UserConstructionScript`)